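; Quest manager actor that adds quests to the game and tracks which one is currently selected.
; AddNewQuest rejects invalid or duplicate classes, spawns an actor per quest, sets up its starting goals and links it to a new HUD list widget.
; The first quest, or one flagged to start directly, goes through SelectNewQuest, which updates the previous and new quest widgets.
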(event `OnSwitch_SubQuests`)

(fn `Add_New_Quest`
  (params (Quest_Class :type "/Game/QuestSystem/BluePrints/Actors/Quest_Actors/BP_MasterQuest Class Reference") (`Directly_Start?` :type Boolean))
  (returns (`Success?` :type Boolean))
  (locals (Local_Class :type "/Game/QuestSystem/BluePrints/Actors/Quest_Actors/BP_MasterQuest Class Reference") (`Start?` :type Boolean) (Local_Quest_Actor :type "/Game/QuestSystem/BluePrints/Actors/Quest_Actors/BP_MasterQuest Object Reference"))
  (bind _local_quest_actor (`local.Local_Quest_Actor`))
  (bind _local_quest_actor_2 (`local.Local_Quest_Actor`))
  (set `local.Local_Class` Quest_Class)
  (set `local.Start?` `Directly_Start?`)
  (if (and (`KismetSystemLibrary.IsValidClass` Quest_Class) (not (`KismetArrayLibrary.Array_Contains` (`self.All_Quest_Classes`) Quest_Class)))
    (`KismetArrayLibrary.Array_Add` (`self.All_Quest_Classes`) (`local.Local_Class`))
    (bind _returnvalue (`|SpawnActorFromClass` (`local.Local_Class`) (`KismetMathLibrary.MakeTransform` (0.0 0.0 0.0)) "AlwaysSpawn" "OverrideRootScale"))
    (bind _output_get (set `local.Local_Quest_Actor` _returnvalue))
    (`KismetArrayLibrary.Array_Add` (`self.Quest_Actors`) _output_get)
    (`/Game/QuestSystem/BluePrints/Actors/Quest_Actors/BP_MasterQuest.Setup_Strating_Goals` _local_quest_actor_2)
    (bind _widget (`/Game/QuestSystem/Widgets/HUD.Add_Quest_to_List` (`self.HUD`) _local_quest_actor_2))
    (bind _output_get_2 (set `/Game/QuestSystem/BluePrints/Actors/Quest_Actors/BP_MasterQuest.Quest_Widget` _widget (`local.Local_Quest_Actor`)))
    (`/Game/QuestSystem/Widgets/Quest_Widget.Update_Quest` _output_get_2)
    (if (or (`local.Start?`) (<= (`KismetArrayLibrary.Array_Length` (`self.Quest_Actors`)) 1))
      (`self.Select_New_Quest` _local_quest_actor (`KismetArrayLibrary.Array_Get` (`/Game/QuestSystem/Widgets/Quest_Widget.SubGoal_Widgets` (`/Game/QuestSystem/BluePrints/Actors/Quest_Actors/BP_MasterQuest.Quest_Widget` _local_quest_actor)))))
    (return true)
    (else
      (return false))))

(fn `Select_New_Quest`
  (params (Quest :type "/Game/QuestSystem/BluePrints/Actors/Quest_Actors/BP_MasterQuest Object Reference") (Sub_Goal :type "/Game/QuestSystem/Widgets/SubGoal_Widget Object Reference"))
  (bind _current_quest (`self.Current_Quest`))
  (bind _quest_widget (`/Game/QuestSystem/BluePrints/Actors/Quest_Actors/BP_MasterQuest.Quest_Widget` _current_quest))
  (`/Engine/EditorBlueprintResources/StandardMacros.IsValid` _current_quest
    (:`Is Valid`
      (`Widget.SetIsEnabled` (`/Game/QuestSystem/Widgets/Quest_Widget.QuestName` _quest_widget) false)
      (`/Game/QuestSystem/Widgets/Quest_Widget.Select_SubGoal` _quest_widget null))
    (:`Is Not Valid`
      _))
  (bind _output_get (set `self.Current_Quest` Quest))
  (`/Game/QuestSystem/Widgets/Quest_Widget.On_Quest_Selected` (`/Game/QuestSystem/BluePrints/Actors/Quest_Actors/BP_MasterQuest.Quest_Widget` _output_get) Sub_Goal)
  (return))

(fn `UserConstructionScript`)