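; BP_MasterQuest is a quest actor, apparently a base for specific quests, that tracks which subgoals in its QuestInfo are active.
; Setup_Strating_Goals seeds the current indices from the starting subgoal indices, and Update_SubGoals rebuilds CurrentGoals from those indices.
; Goto_Next_SubGoal replaces all current goals with the one after the highest active index, returning false when none remain.
; The event graph and construction script are empty.
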(fn `Goto_Next_SubGoal`
  (returns (`Success?` :type Boolean))
  (locals (Next_Index :type Integer))
  (bind _current_goal_indices (`self.Current_Goal_Indices`))
  (bind _returnvalue (+ (`.MaxValue` (`KismetMathLibrary.MaxOfIntArray` (`self.Current_Goal_Indices`))) 1))
  (if (<= _returnvalue (`KismetArrayLibrary.Array_LastIndex` (`.SubGoal_28_1F01CA68497C81A86DEDA0A867445EFE` (break `/Game/QuestSystem/BluePrints/Structures/S_Quest_Info` (`self.Quest_Info`)))))
    (set `local.Next_Index` _returnvalue)
    (`KismetArrayLibrary.Array_Clear` _current_goal_indices)
    (`KismetArrayLibrary.Array_Add` _current_goal_indices (`local.Next_Index`))
    (`self.Update_SubGoals`)
    (return true)
    (else
      (return false))))

(fn `Setup_Strating_Goals`
  (`KismetArrayLibrary.Array_Clear` (`self.Current_Goal_Indices`))
  (set `self.Current_Goal_Indices` (`self.Starting_SubGoal_indices`))
  (`self.Update_SubGoals`)
  (return))

(fn `Update_SubGoals`
  (`KismetArrayLibrary.Array_Clear` (`self.Current_Goals`))
  (for _array_element (`self.Current_Goal_Indices`)
    (`KismetArrayLibrary.Array_Add` (`self.Current_Goals`) (`KismetArrayLibrary.Array_Get` (`.SubGoal_28_1F01CA68497C81A86DEDA0A867445EFE` (break `/Game/QuestSystem/BluePrints/Structures/S_Quest_Info` (`self.Quest_Info`))) _array_element)))
  (return))

(fn `UserConstructionScript`)